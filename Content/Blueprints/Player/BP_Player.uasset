(event `self.ReceiveBeginPlay`
  (bind _returnvalue (`GameplayStatics.GetPlayerController` 0))
  (`EnhancedInputSubsystemInterface.AddMappingContext` (pcsubsystem `EnhancedInputLocalPlayerSubsystem` _returnvalue) "/Game/Inputs/IMC_PlayerInputs.IMC_PlayerInputs" 0 (struct))
  (bind _returnvalue_2 (`|CreateWidget` "/Game/Blueprints/Widgets/UW_GameUI.UW_GameUI_C" _returnvalue))
  (bind _output_get (set `self.Widget` _returnvalue_2))
  (`UserWidget.AddToViewport` _output_get 0)
  (`/Game/Blueprints/Widgets/UW_GameUI.SetDeliveryRemaining` _output_get))

(event `self.ReceiveHit`
  (params (MyComp :type "PrimitiveComponent Object Reference") (Other :type "Actor Object Reference") (OtherComp :type "PrimitiveComponent Object Reference") (bSelfMoved :type Boolean) (HitLocation :type "Vector Structure") (HitNormal :type "Vector Structure") (NormalImpulse :type "Vector Structure") (Hit :type "HitResult Structure (by ref)"))
  (if (`self.CanCollide` Other)
    (`self.Collision` HitNormal)))

(event `self.ReceiveTick`
  (params (DeltaSeconds :type "Float (single-precision)"))
  (`self.Movements`)
  (`self.Turn`))

(event `EnhancedInput|/Game/Inputs/IA_Accelerate`
  (params (ActionValue :type Boolean) (ElapsedSeconds :type "Float (double-precision)") (TriggeredSeconds :type "Float (double-precision)") (InputAction :type "InputAction Object Reference" :default "/Game/Inputs/IA_Accelerate.IA_Accelerate"))
  (bind _carcomponent (`self.CarComponent`))
  (:`Started`
    (set `CarComponent.isAccelerating` true _carcomponent)
    (set `CarComponent.isDeccelerating` false _carcomponent))
  (:`Completed`
    (set `CarComponent.isAccelerating` false (`self.CarComponent`))))

(event `self.ReceiveActorBeginOverlap`
  (params (OtherActor :type "Actor Object Reference"))
  (if (`self.ActorHasTag` OtherActor "DeliveryZone")
    (bind _asbp_delivery_zone (cast `/Game/Blueprints/DeliveryZone/BP_DeliveryZone` OtherActor))
    (`self.DeliverInZone` _asbp_delivery_zone)
    (elif (and (`self.ActorHasTag` OtherActor "End") (== (`self.DeliveryPointsRemaining`) 0.0))
      (`self.Finish Game`))))

(event `EnhancedInput|/Game/Inputs/IA_LookAround`
  (params (ActionValue :type "Float (double-precision)") (ElapsedSeconds :type "Float (double-precision)") (TriggeredSeconds :type "Float (double-precision)") (InputAction :type "InputAction Object Reference" :default "/Game/Inputs/IA_LookAround.IA_LookAround"))
  (:`Triggered`
    (`SceneComponent.K2_AddLocalRotation` (`self.SpringArm`) (`KismetMathLibrary.MakeRotator` 0.0 0.0 ActionValue) false false)))

(event `EnhancedInput|/Game/Inputs/IA_ActivateDrift`
  (params (ActionValue :type Boolean) (ElapsedSeconds :type "Float (double-precision)") (TriggeredSeconds :type "Float (double-precision)") (InputAction :type "InputAction Object Reference" :default "/Game/Inputs/IA_ActivateDrift.IA_ActivateDrift"))
  (bind _floatingpawnmovement (`self.FloatingPawnMovement`))
  (:`Triggered`
    (set `FloatingPawnMovement.TurningBoost` 0.0 _floatingpawnmovement))
  (:`Completed`
    (set `FloatingPawnMovement.TurningBoost` 6.0 _floatingpawnmovement)))

(event `EnhancedInput|/Game/Inputs/AI_Deccelerate`
  (params (ActionValue :type Boolean) (ElapsedSeconds :type "Float (double-precision)") (TriggeredSeconds :type "Float (double-precision)") (InputAction :type "InputAction Object Reference" :default "/Game/Inputs/AI_Deccelerate.AI_Deccelerate"))
  (bind _carcomponent (`self.CarComponent`))
  (:`Started`
    (set `CarComponent.isDeccelerating` true _carcomponent)
    (set `CarComponent.isAccelerating` false _carcomponent))
  (:`Completed`
    (set `CarComponent.isDeccelerating` false (`self.CarComponent`))))

(event `EnhancedInput|/Game/Inputs/IA_Lift`
  (params (ActionValue :type Boolean) (ElapsedSeconds :type "Float (double-precision)") (TriggeredSeconds :type "Float (double-precision)") (InputAction :type "InputAction Object Reference" :default "/Game/Inputs/IA_Lift.IA_Lift"))
  (bind (_returnvalue_x _returnvalue_y _returnvalue_z) (`KismetMathLibrary.BreakVector` (`self.K2_GetActorLocation`)))
  (bind (_returnvalue_roll _returnvalue_pitch _returnvalue_yaw) (`KismetMathLibrary.BreakRotator` (`self.K2_GetActorRotation`)))
  (:`Started`
    (`self.K2_SetActorLocationAndRotation` (`KismetMathLibrary.MakeVector` _returnvalue_x _returnvalue_y (+ _returnvalue_z 10.0)) (`KismetMathLibrary.MakeRotator` 0.0 0.0 _returnvalue_yaw))))

(event `EnhancedInput|/Game/Inputs/IA_Turn`
  (params (ActionValue :type "Float (double-precision)") (ElapsedSeconds :type "Float (double-precision)") (TriggeredSeconds :type "Float (double-precision)") (InputAction :type "InputAction Object Reference" :default "/Game/Inputs/IA_Turn.IA_Turn"))
  (:`Triggered`
    (set `self.Turning` true)
    (set `self.TurnAngle` (`KismetMathLibrary.FClamp` (+ (`self.TurnAngle`) (* (* ActionValue (`KismetMathLibrary.SignOfFloat` (`CarComponent.currentSpeed` (`self.CarComponent`)))) 0.05)) -1.0)))
  (:`Completed`
    (set `self.Turning` false)
    (for _ (range 21)
      (`KismetSystemLibrary.Delay` 0.2)
      (bind _finished (`self.TurnReturnToZero`))
      (if (not _finished)
        (set `self.TurnAngle` 0.0)
        (break)))))

(fn `CanCollide`
  (params (`Collision actor` :type "Actor Object Reference"))
  (returns (canCollide :type Boolean))
  (bind _currentspeed (`CarComponent.currentSpeed` (`self.CarComponent`)))
  (return (and (not (`self.ActorHasTag` `Collision actor` "Floor")) (or (> _currentspeed 0.3) (< _currentspeed -0.3)))))

(fn `Collision`
  (params (Normal :type "Vector Structure"))
  (bind _floatingpawnmovement (`self.FloatingPawnMovement`))
  (set `CarComponent.currentSpeed` 0.0 (`self.CarComponent`))
  (`PrimitiveComponent.SetPhysicsLinearVelocity` (`self.Vespa`) (- (`MovementComponent.Velocity` _floatingpawnmovement) (* (+ 1.0 (`self.RestitutionCoefition`)) (`KismetMathLibrary.Dot_VectorVector` (`MovementComponent.Velocity` _floatingpawnmovement) Normal) Normal)) true "None"))

(fn `DeliverInZone`
  (params (DeliverZone :type "/Game/Blueprints/DeliveryZone/BP_DeliveryZone Object Reference"))
  (if (not (`/Game/Blueprints/DeliveryZone/BP_DeliveryZone.WasDelivered` DeliverZone))
    (`/Game/Blueprints/DeliveryZone/BP_DeliveryZone.Deliver` DeliverZone)
    (bind _output_get (set `self.DeliveryPointsRemaining` (- (`self.DeliveryPointsRemaining`) 1.0)))
    (`/Game/Blueprints/Widgets/UW_GameUI.SetDeliveryRemaining` (`self.Widget`))
    (if (== _output_get 0.0)
      (`/Game/Blueprints/Widgets/UW_GameUI.Set Finish Text` (`self.Widget`)))))

(fn `Finish Game`
  (`GameplayStatics.OpenLevelBySoftObjectPtr` "/Game/Level/L_Win.L_Win")
  (set `PlayerController.bShowMouseCursor` true (`GameplayStatics.GetPlayerController` 0)))

(fn `Movements`
  (`self.AddMovementInput` (`SceneComponent.GetForwardVector` (`self.Vespa`)) (`CarComponent.currentSpeed` (`self.CarComponent`)) true))

(fn `Turn`
  (`self.K2_AddActorWorldRotation` (`KismetMathLibrary.MakeRotator` 0.0 0.0 (* (`self.TurnAngle`) (`KismetMathLibrary.Abs` (`CarComponent.currentSpeed` (`self.CarComponent`)))))))

(fn `TurnReturnToZero`
  (returns (Finished :type Boolean))
  (if (`self.Turning`)
    (return true)
    (elif (> (`self.TurnAngle`) 0.0)
      (bind _output_get (set `self.TurnAngle` (- 0.0 0.1)))
      (if (< _output_get 0.0)
        (set `self.TurnAngle` 0.0)
        (return true)
        (else
          (return false)))
      (else
        (bind _output_get_2 (set `self.TurnAngle` (+ 0.0 0.1)))
        (if (> _output_get_2 0.0)
          (set `self.TurnAngle` 0.0)
          (return true)
          (else
            (return false)))))))

(fn `UserConstructionScript`)