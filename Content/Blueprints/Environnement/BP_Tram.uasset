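; BP_Tram is an environment tram that travels along a short path and pauses briefly at an intermediate stop.
; The construction script feeds the InterpToMovement component three relative control points: the origin, Stop and LastStep.
; Each tick compares the location with the start position offset by Stop.X along the mesh's forward vector.
; Near that point, it disables the movement component's tick, waits two seconds, then re-enables it.
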(event `self.ReceiveBeginPlay`
  (set `self.StartPosition` (`self.K2_GetActorLocation`)))

(event `self.ReceiveTick`
  (params (DeltaSeconds :type "Float (single-precision)"))
  (if (== (`self.K2_GetActorLocation`) (+ (`self.StartPosition`) (* (`SceneComponent.GetForwardVector` (`self.StaticMesh`)) (.x (`self.Stop`)))) :`ErrorTolerance` 4.0)
    (`ActorComponent.SetComponentTickEnabled` (`self.InterpToMovement`) false)
    (`KismetSystemLibrary.Delay` 2.0)
    (`ActorComponent.SetComponentTickEnabled` (`self.InterpToMovement`) true)))

(fn `UserConstructionScript`
  (bind _interptomovement (`self.InterpToMovement`))
  (`InterpToMovementComponent.AddControlPointPosition` (`self.InterpToMovement`) (0.0 0.0 0.0) true)
  (`InterpToMovementComponent.AddControlPointPosition` _interptomovement (`self.Stop`) true)
  (`InterpToMovementComponent.AddControlPointPosition` _interptomovement (`self.LastStep`) true))